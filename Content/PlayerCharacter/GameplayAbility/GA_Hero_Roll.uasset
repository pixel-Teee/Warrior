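; Hero dodge-roll gameplay ability that plays a roll montage steered by motion warping toward the last movement input.
; After a brief delay, it caches the input direction and sets it as the rotation warp target.
; A downward trace from a point ahead sets the location warp target, with persistent debug drawing and no hit check.
; The ability ends when the montage completes, blends out, is interrupted or is cancelled.
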(event `self.K2_ActivateAbility`
  (`KismetSystemLibrary.Delay` 0.05)
  (`self.ComputeRollDirectionDistance`)
  (`AbilityTask_PlayMontageAndWait.CreatePlayMontageAndWaitProxy` "None" "/Game/PlayerCharacter/Montages/AM_Hero_Roll.AM_Hero_Roll"
    (:`OnCompleted`
      _)
    (:`OnBlendOut`
      _)
    (:`OnInterrupted`
      _)
    (:`OnCancelled`
      _))
  (`self.K2_EndAbility`))

(fn `ComputeRollDirectionDistance`
  (locals (CachedRollingDirection :type "Vector Structure" :default (0.0 0.0 0.0)))
  (bind _returnvalue (+ (`Actor.K2_GetActorLocation` (`self.GetHeroCharacterFromActorInfo`)) (* (`local.CachedRollingDirection`) 500.0)))
  (set `local.CachedRollingDirection` (`KismetMathLibrary.Normal` (`Pawn.GetLastMovementInputVector` (`self.GetHeroCharacterFromActorInfo`))))
  (`|ExecutionSequence`
    (:`then_0`
      (`MotionWarpingComponent.AddOrUpdateWarpTargetFromLocationAndRotation` (`WarriorBaseCharacter.MotionWarpingComponent` (`self.GetHeroCharacterFromActorInfo`)) "RollingDirection" (0.0 0.0 0.0) (`KismetMathLibrary.MakeRotFromX` (`local.CachedRollingDirection`))))
    (:`then_1`
      (bind _outhit (`KismetSystemLibrary.LineTraceSingleForObjects` :`Start` _returnvalue :`End` (+ _returnvalue (* (* (`Actor.GetActorUpVector` (`self.GetHeroCharacterFromActorInfo`)) -1.0) 500.0)) :`ObjectTypes` (`self.Object Types`) :`DrawDebugType` "Persistent"))
      (`MotionWarpingComponent.AddOrUpdateWarpTargetFromLocation` (`WarriorBaseCharacter.MotionWarpingComponent` (`self.GetHeroCharacterFromActorInfo`)) "RollTargetLocation" (`.ImpactPoint` (`GameplayStatics.BreakHitResult` _outhit))))))